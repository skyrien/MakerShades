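; VR pawn that spawns and removes BP_Sphere actors with the motion controller triggers or keyboard keys.
; Right trigger or K spawns a sphere at the right controller's world location, further transformed by player character 0's actor transform, and adds it to an Objects array.
; Left trigger or T destroys and removes the array entry at index Length, one past the last element rather than the newest sphere.
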(event `Key|T`
  (params (Key :type "Key Structure" :default "AnyKey"))
  (bind _objects (`self.Objects`))
  (:`Pressed`
    (`self.K2_DestroyActor` (`KismetArrayLibrary.Array_Get` _objects (`KismetArrayLibrary.Array_Length` _objects)) :!label _label)
    (`KismetArrayLibrary.Array_RemoveItem` _objects null)))

(event `Key|K`
  (params (Key :type "Key Structure" :default "AnyKey"))
  (:`Pressed`
    (bind _returnvalue (`|SpawnActorFromClass` "/Game/MakerShades/Blueprints/BP_Sphere.BP_Sphere_C" (`KismetMathLibrary.Conv_VectorToTransform` (`KismetMathLibrary.TransformLocation` (`self.GetTransform` (`GameplayStatics.GetPlayerCharacter` 0)) (`SceneComponent.K2_GetComponentLocation` (`self.MotionControllerRight`)))) "Undefined" "OverrideRootScale" :!label _label_2))
    (`KismetArrayLibrary.Array_Add` (`self.Objects`) _returnvalue)))

(event `Key|MotionController_Left_Trigger`
  (params (Key :type "Key Structure" :default "AnyKey"))
  (:`Pressed`
    (goto _label)))

(event `Key|MotionController_Right_Trigger`
  (params (Key :type "Key Structure" :default "AnyKey"))
  (:`Pressed`
    (goto _label_2)))

(fn `UserConstructionScript`)